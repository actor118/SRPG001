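; BP_Pawn is a player pawn acting as a camera rig with keyboard movement and rotation and clamped mouse-wheel spring-arm zoom.
; BeginPlay adds the IM_Zoom mapping context and seeds desired location, rotation and zoom, which Enhanced Input events then adjust.
; Tick interpolates zoom and rotation toward their targets, but its VInterpTo starts from LocationDesired toward the current location, so movement is barely smoothed.
; A separate MouseMiddleScroll graph sets arm length directly.
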(event `self.ReceiveBeginPlay`
  (bind `_as玩家控制器` (cast `PlayerController` (`self.GetController`)))
  (bind _returnvalue (pcsubsystem `EnhancedInputLocalPlayerSubsystem` `_as玩家控制器`))
  (`/Engine/EditorBlueprintResources/StandardMacros.IsValid` _returnvalue
    (:`Is Valid`
      (`EnhancedInputSubsystemInterface.AddMappingContext` _returnvalue "/Game/BluePrints/Input/IM_Zoom.IM_Zoom" 0 (struct))
      (set `self.LocationDesired` (`self.K2_GetActorLocation`))
      (set `self.ZoomDesired` (`SpringArmComponent.TargetArmLength` (`self.SpringArm`)))
      (set `self.RotationDesired` (`self.K2_GetActorRotation`)))))

(event `EnhancedInput|/Game/BluePrints/Input/IA_KB_Move_H`
  (params (ActionValue :type "Float (double-precision)") (ElapsedSeconds :type "Float (double-precision)") (TriggeredSeconds :type "Float (double-precision)") (InputAction :type "InputAction Object Reference" :default "/Game/BluePrints/Input/IA_KB_Move_H.IA_KB_Move_H"))
  (:`Triggered`
    (set `self.LocationDesired` (+ (`self.LocationDesired`) (* (`self.GetActorForwardVector`) (* ActionValue (`self.MoveDistance`)))))))

(event `EnhancedInput|/Game/BluePrints/Input/IA_Mouse_Wheel`
  (params (ActionValue :type "Float (double-precision)") (ElapsedSeconds :type "Float (double-precision)") (TriggeredSeconds :type "Float (double-precision)") (InputAction :type "InputAction Object Reference" :default "/Game/BluePrints/Input/IA_Mouse_Wheel.IA_Mouse_Wheel"))
  (:`Triggered`
    (set `self.ZoomDesired` (`KismetMathLibrary.FClamp` (+ (`self.ZoomDesired`) (* ActionValue (`self.Wheel Distance1`))) 500.0 3000.0))))

(event `EnhancedInput|/Game/BluePrints/Input/IA_KB_Move_V`
  (params (ActionValue :type "Float (double-precision)") (ElapsedSeconds :type "Float (double-precision)") (TriggeredSeconds :type "Float (double-precision)") (InputAction :type "InputAction Object Reference" :default "/Game/BluePrints/Input/IA_KB_Move_V.IA_KB_Move_V"))
  (:`Triggered`
    (set `self.LocationDesired` (+ (`self.LocationDesired`) (* (`self.GetActorRightVector`) (* ActionValue (`self.MoveDistance`)))))))

(event `EnhancedInput|/Game/BluePrints/Input/IA_KB_Rotation`
  (params (ActionValue :type "Float (double-precision)") (ElapsedSeconds :type "Float (double-precision)") (TriggeredSeconds :type "Float (double-precision)") (InputAction :type "InputAction Object Reference" :default "/Game/BluePrints/Input/IA_KB_Rotation.IA_KB_Rotation"))
  (:`Started`
    (set `self.RotationDesired` (`KismetMathLibrary.ComposeRotators` (`self.RotationDesired`) (* (`self.RotationDistance`) ActionValue)))))

(event `self.ReceiveTick`
  (params (DeltaSeconds :type "Float (single-precision)"))
  (bind _springarm (`self.SpringArm`))
  (set `SpringArmComponent.TargetArmLength` (`KismetMathLibrary.FInterpTo` (`SpringArmComponent.TargetArmLength` _springarm) (`self.ZoomDesired`) DeltaSeconds 1.0) _springarm)
  (`self.K2_SetActorLocation` (`KismetMathLibrary.VInterpTo` (`self.LocationDesired`) (`self.K2_GetActorLocation`) DeltaSeconds 1.0))
  (`self.K2_SetActorRotation` (`KismetMathLibrary.RInterpTo` (`self.K2_GetActorRotation`) (`self.RotationDesired`) DeltaSeconds 2.0)))

(fn `Mouse Middle Scroll`
  (bind _springarm (`self.SpringArm`))
  (set `self.ZoomDesired` (`self.GetInputAxisKeyValue`))
  (set `SpringArmComponent.TargetArmLength` (`KismetMathLibrary.FClamp` (- (`SpringArmComponent.TargetArmLength` _springarm) (* (`self.ZoomDesired`) (`self.Wheel Distance1`))) 500.0 3000.0) _springarm))

(fn `UserConstructionScript`)